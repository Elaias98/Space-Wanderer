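; BP_asteroide is an asteroid actor that moves each tick by a velocity set through SetearVelocidadM1 and destroys itself after a 12-second delay.
; When its DañoYDestroy component begins an overlap, it sends the VidaPersonaje interface message to the other actor.
; When the overlap ends, it sends DestruitMeteoro, destroys itself and spawns four fragment variants at its transform.
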(event `self.ReceiveTick`
  (params (DeltaSeconds :type "Float (single-precision)"))
  (`self.K2_AddActorLocalOffset` (`self.VelocidadMeteoro1`))
  (`KismetSystemLibrary.Delay` 12.0)
  (`self.K2_DestroyActor`))

(event `self.DañoYDestroy.OnComponentBeginOverlap`
  (params (OverlappedComponent :type "PrimitiveComponent Object Reference") (OtherActor :type "Actor Object Reference") (OtherComp :type "PrimitiveComponent Object Reference") (OtherBodyIndex :type Integer) (bFromSweep :type Boolean) (SweepResult :type "HitResult Structure (by ref)"))
  (message `/Game/Blueprint/Tiles/Interface/BPI_VidaPersonaje.VidaPersonaje` OtherActor))

(event `self.DañoYDestroy.OnComponentEndOverlap`
  (params (OverlappedComponent :type "PrimitiveComponent Object Reference") (OtherActor :type "Actor Object Reference") (OtherComp :type "PrimitiveComponent Object Reference") (OtherBodyIndex :type Integer))
  (message `/Game/Blueprint/Tiles/Interface/BPI_DestruirObstaculo.DestruitMeteoro` OtherActor)
  (`self.K2_DestroyActor`)
  (`KismetSystemLibrary.PrintString` "Hello" true true (struct :`R` 1.0 :`G` 0.042226 :`A` 1.0) 800000.0 "None")
  (`|SpawnActorFromClass` "/Game/Blueprint/BP_fragmento.BP_fragmento_C" (`self.GetTransform`) "Undefined" "MultiplyWithRoot" null null)
  (`|SpawnActorFromClass` "/Game/Blueprint/BP_fragmento_Child.BP_fragmento_Child_C" (`self.GetTransform`) "Undefined" "MultiplyWithRoot" null null)
  (`|SpawnActorFromClass` "/Game/Blueprint/BP_fragmento_Child1.BP_fragmento_Child1_C" (`self.GetTransform`) "Undefined" "MultiplyWithRoot" null null)
  (`|SpawnActorFromClass` "/Game/Blueprint/BP_fragmento_Child2.BP_fragmento_Child2_C" (`self.GetTransform`) "Undefined" "MultiplyWithRoot" null null))

(event `self.DañoYDestroy.OnComponentHit`
  (params (HitComponent :type "PrimitiveComponent Object Reference") (OtherActor :type "Actor Object Reference") (OtherComp :type "PrimitiveComponent Object Reference") (NormalImpulse :type "Vector Structure") (Hit :type "HitResult Structure (by ref)")))

(fn `Setear Velocidad M1`
  (params (`Vel.Meteoro1` :type "Vector Structure"))
  (set `self.VelocidadMeteoro1` `Vel.Meteoro1`))

(fn `UserConstructionScript`)