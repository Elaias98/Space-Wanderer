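; Meteor spawner actor that drifts back and forth while offering functions to spawn two asteroid types at its location.
; A looping timer flips the ArribaAbajo flag, which selects the positive or negative local offset applied each Tick.
; Tick also rerolls a random speed multiplier, which VelocidadMeteoros applies to its input.
; SpawnMeteoros1 and 2 pass a given velocity to BP_asteroide and BP_asteroide2; nothing in this Blueprint calls them.
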(event `self.ReceiveBeginPlay`
  (`KismetSystemLibrary.K2_SetTimerDelegate` (delegate `Arriba/Abajo`) 10.0 true))

(event `Arriba/Abajo`
  (set `self.ArribaAbajo` (not (`self.ArribaAbajo`)))
  (`KismetSystemLibrary.K2_ClearTimer` null))

(event `self.ReceiveTick`
  (params (DeltaSeconds :type "Float (single-precision)"))
  ;[1 1 1] Damos un rango aleatorio al multiplicador para variar las velocidades de los asteroides
  ;
  ; Lo agrego al Event Tick para que se actuelizen los valores de la velocidad de los meteoros
  (set `self.MultiplicadorVelocidad` (`KismetMathLibrary.RandomFloatInRange` 20.0 50.0))
  (if (`self.ArribaAbajo`)
    (`self.K2_AddActorLocalOffset` (`self.VelocidadSpawnPositivo`))
    (else
      (`self.K2_AddActorLocalOffset` (`self.VelocidadSpawnNegativo`)))))

(fn `SpawnMeteoros1`
  (params (IngresoVelMeteoro1 :type "Vector Structure"))
  (`|SpawnActorFromClass` "/Game/Blueprint/BP_asteroide.BP_asteroide_C" (`KismetMathLibrary.MakeTransform` (`self.K2_GetActorLocation`)) "Undefined" "MultiplyWithRoot" null IngresoVelMeteoro1 null))

(fn `SpawnMeteoros2`
  (params (VelMeteoro2 :type "Vector Structure"))
  (locals (NewLocalVar :type "Transform Structure"))
  (`|SpawnActorFromClass` "/Game/Blueprint/BP_asteroide2.BP_asteroide2_C" (`KismetMathLibrary.MakeTransform` (`self.K2_GetActorLocation`)) "Undefined" "MultiplyWithRoot" null VelMeteoro2 0.0 null))

(fn `UserConstructionScript`)

(fn `VelocidadMeteoros`
  (params (Input :type "Vector Structure"))
  (returns (Resultante :type "Vector Structure"))
  (return (* Input (`self.MultiplicadorVelocidad`))))