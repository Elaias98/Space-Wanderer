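; BP_FInal is a player character that flies on the X/Z plane, shoots projectiles and loses health.
; BeginPlay sets Flying mode and adds the Enhanced Input mapping, which drives movement, stopping on release, and BP_Proyectil spawning gated by SeDisparo.
; VidaPersonaje decrements Vida after a delay, then at zero destroys the actor and opens TEST2D.
; Tick prints Vida, while the asteroid speed-up event is an empty stub with disconnected draft logic.
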(event `self.ReceiveTick`
  (params (DeltaSeconds :type "Float (single-precision)"))
  (`KismetSystemLibrary.PrintString` (`KismetStringLibrary.Concat_StrStr` "Vida Del Personaje:" (`KismetStringLibrary.Conv_DoubleToString` (`self.Vida`))) true true (struct :`R` 0.002694 :`G` 1.0 :`B` 0.065134 :`A` 1.0) 4000.0 "1"))

(event `self.ReceiveBeginPlay`
  ;[1 1 1] INPUTS Y MAPS CONTROLLERS
  (`CharacterMovementComponent.SetMovementMode` (`self.CharacterMovement`) "MOVE_Flying" 0)
  (bind _asplayer_controller (cast `PlayerController` (`self.GetController`)))
  (message `EnhancedInputSubsystemInterface.AddMappingContext` (pcsubsystem `EnhancedInputLocalPlayerSubsystem` _asplayer_controller) "/Game/InputMapContex/IMP_PRUEBA.IMP_PRUEBA" 0 (struct)))

(event `/Game/Blueprint/Tiles/Interface/BPI_AumentarVelocidad.SubirVelocidad`
  ;[1 1 1] Aumentar velocidad al acercarse un asteroide
)

(event `EnhancedInput|/Game/Inputs/IA_movimiento`
  (params (ActionValue :type "Vector2D Structure") (ElapsedSeconds :type "Float (double-precision)") (TriggeredSeconds :type "Float (double-precision)") (InputAction :type "InputAction Object Reference" :default "/Game/Inputs/IA_movimiento.IA_movimiento"))
  ;[1 1 1] Movimiento Izquierda Derecha
  (:`Triggered`
    (`self.AddMovementInput` (1.0 0.0 0.0) ActionValue_X)
    (`self.AddMovementInput` (0.0 0.0 1.0) ActionValue_Y))
  (:`Completed`
    (`MovementComponent.StopMovementImmediately` (`self.CharacterMovement`))))

(event `/Game/Blueprint/Tiles/Interface/BPI_VidaPersonaje.VidaPersonaje`
  ;[1 1 1] VIDA PERSONAJE
  (`KismetSystemLibrary.Delay` 1.5)
  (set `self.Vida` (- (`self.Vida`) 1.0))
  (if (== 0.0 (`self.Vida`))
    (`self.K2_DestroyActor`)
    (if (<= (`self.Vida`) 0.0)
      (`GameplayStatics.OpenLevel` "TEST2D"))))

(event `EnhancedInput|/Game/Inputs/IA_Shoot`
  (params (ActionValue :type Boolean) (ElapsedSeconds :type "Float (double-precision)") (TriggeredSeconds :type "Float (double-precision)") (InputAction :type "InputAction Object Reference" :default "/Game/Inputs/IA_Shoot.IA_Shoot"))
  (bind _returnvalue (`self.GetTransform`))
  (:`Started`
    (if (`self.SeDisparo?`)
      (`|SpawnActorFromClass` "/Game/Blueprint/BP_Proyectil.BP_Proyectil_C" (`KismetMathLibrary.MakeTransform` (`KismetMathLibrary.MakeVector` (+ (.x (.location _returnvalue)) 90.0) (+ (.y (.location _returnvalue)) 0.0) (.z (.location _returnvalue)))) "Undefined" "MultiplyWithRoot" null null))))

(fn `UserConstructionScript`)